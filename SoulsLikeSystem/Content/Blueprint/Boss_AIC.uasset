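; Boss_AIC is the AI controller for the boss, starting its behavior tree when it possesses a pawn.
; On possess it runs Boss_BT, then seeds the blackboard with starting phase, health percentage and the controlled pawn as SelfActor.
; It also stores the first player character, cast to Player_BP, as TargetActor, leaving the target unset if that cast fails.
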(event EventPossess
  (params (PossessedPawn :type Pawn%20Object%20Reference))
  (bind _returnvalue (AI|GetBlackboard 0))
  ;[0.15 0.15 0.15 0.5] Activate Behavior Tree
  (AI|RunBehaviorTree "/Game/BehaviorTree/Boss_BT.Boss_BT")
  (Class|BlackboardComponent|SetValueasInt _returnvalue (Utilities|Name|MakeLiteralName "CurrentPhase") 1)
  (AI|Components|Blackboard|SetValueasFloat _returnvalue (Utilities|Name|MakeLiteralName "HealthPercentage") 1e+02)
  (AI|Components|Blackboard|SetValueasObject _returnvalue (Utilities|Name|MakeLiteralName "SelfActor") (Pawn|GetControlledPawn))
  (bind _asplayer_bp (Utilities|Casting|CastToPlayer_BP (Game|GetPlayerCharacter 0)))
  (AI|Components|Blackboard|SetValueasObject _returnvalue (Utilities|Name|MakeLiteralName "TargetActor") _asplayer_bp))

(fn ConstructionScript)