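; Player character Blueprint with Enhanced Input movement, look, running, lock-on targeting and a directional roll.
; Targeting sphere-traces along the camera for a Pawn, flags Player_ABP as locked, and Tick steers control and actor rotation toward it.
; Rolls turn toward camera-relative input and play a montage behind a DoOnce, clearing IsRolling shortly before it ends so target facing resumes.
; BeginPlay also loops an enemy Level Sequence on a timer.
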(event Custom|PlayMyAnimation
  ;[0.15 0.15 0.15 0.5] Custom event
  (Sequencer|Player|Play (Variables|Default|GetNewVar_0) :!class /Script/MovieScene.MovieSceneSequencePlayer))

(event Custom|SetIsRollingDelay
  ;[0.15 0.15 0.15 0.5] Set IsRolling False before roll animation ends
  (Utilities|FlowControl|Delay (- (Variables|Default|GetRollAnimetionTime) 0.3))
  (Variables|Default|SetIsRolling false))

(event Custom|DetectMovementKeys
  (bind _currentmovementkeys (Variables|Default|GetCurrentMovementKeys))
  ;[0.15 0.15 0.15 0.5] Detect last movement key
  (for (_array_element _array_index) (Variables|Default|GetMovementKeys)
    (if (Game|Player|IsInputKeyDown (Game|GetPlayerController 0) (Utilities|Array|Get(acopy) (Variables|Default|GetKey) _array_index))
      (Utilities|Array|SetArrayElem _currentmovementkeys _array_index _array_element)
      (else
        (Utilities|Array|SetArrayElem _currentmovementkeys _array_index "")))))

(event Custom|AdjustCameraForTarget
  (if (Variables|Default|GetIsTargeting)
    _))

(event Custom|UpdateCurrentRotations
  (bind _currentrotations (Variables|Default|GetCurrentRotations))
  ;[0.15 0.15 0.15 0.5] Show current rotations
  (for (_ _array_index) _currentrotations
    (Utilities|Array|SetArrayElem _currentrotations _array_index (+ (.Yaw (Math|Rotator|BreakRotator (Pawn|GetControlRotation :!class /Script/Engine.Pawn))) (Utilities|Array|Get(acopy) (Variables|Default|GetAllRotations) _array_index)))))

(event Input|EnhancedActionEvents|EnhancedInputActionIA_Look
  (params (ActionValue :type Vector%202D%20Structure) (ElapsedSeconds :type Float%20%28double-precision%29) (TriggeredSeconds :type Float%20%28double-precision%29) (InputAction :type Input%20Action%20Object%20Reference :default "/Game/Input/IA_Look.IA_Look"))
  ;[0.15 0.15 0.15 0.5] Camera control
  (Pawn|Input|AddControllerYawInput (.x ActionValue))
  (Pawn|Input|AddControllerPitchInput (* (.y ActionValue) -1.0)))

(event Input|EnhancedActionEvents|EnhancedInputActionIA_Move
  (params (ActionValue :type Vector%202D%20Structure) (ElapsedSeconds :type Float%20%28double-precision%29) (TriggeredSeconds :type Float%20%28double-precision%29) (InputAction :type Input%20Action%20Object%20Reference :default "/Game/Input/IA_Move.IA_Move"))
  (bind _returnvalue (Pawn|GetControlRotation :!class /Script/Engine.Pawn))
  (bind _returnvalue_2 (Game|GetPlayerController 0))
  (bind _returnvalue_3 (Game|GetPlayerController 0))
  ;[0.15 0.15 0.15 0.5] Movement control
  (CallFunction|DetectMovementKeys)
  (Variables|Default|SetCurrentMoveVector (Math|Vector2D|MakeVector2D (.x ActionValue) (.y ActionValue)))
  (Pawn|Input|AddMovementInput (Math|Vector|GetRightVector (Math|Rotator|MakeRotator (.roll _returnvalue) 0.0 (.yaw _returnvalue))) (Math|Float|SelectFloat 0.0 (.x ActionValue) (and (Game|Player|IsInputKeyDown _returnvalue_2 "A") (Game|Player|IsInputKeyDown _returnvalue_2 "D"))) false)
  (Pawn|Input|AddMovementInput (Math|Vector|GetForwardVector (Math|Rotator|MakeRotator 0.0 0.0 (.yaw (Pawn|GetControlRotation :!class /Script/Engine.Pawn)))) (Math|Float|SelectFloat 0.0 (.y ActionValue) (and (Game|Player|IsInputKeyDown _returnvalue_3 "W") (Game|Player|IsInputKeyDown _returnvalue_3 "S"))) false))

(event Input|EnhancedActionEvents|EnhancedInputActionIA_Running
  (params (ActionValue :type Boolean) (ElapsedSeconds :type Float%20%28double-precision%29) (TriggeredSeconds :type Float%20%28double-precision%29) (InputAction :type Input%20Action%20Object%20Reference :default "/Game/Input/IA_Running.IA_Running"))
  (bind _charactermovement (Variables|Character|GetCharacterMovement))
  ;[0.15 0.15 0.15 0.5] Running
  (:Triggered
    (Variables|/Script/Engine.CharacterMovementComponent|SetMaxWalkSpeed _charactermovement 375.0))
  (:Completed
    (Variables|/Script/Engine.CharacterMovementComponent|SetMaxWalkSpeed _charactermovement 275.0)))

(event Input|EnhancedActionEvents|EnhancedInputActionIA_Roll
  (params (ActionValue :type Boolean) (ElapsedSeconds :type Float%20%28double-precision%29) (TriggeredSeconds :type Float%20%28double-precision%29) (InputAction :type Input%20Action%20Object%20Reference :default "/Game/Input/IA_Roll.IA_Roll"))
  (bind _currentmovevector (Variables|Default|GetCurrentMoveVector))
  ;[0.15 0.15 0.15 0.5] Roll system
  (Utilities|FlowControl|DoOnce false :!label _label
    (:Completed
      (if (> (Math|Vector2D|Vector2DLength (Variables|Default|GetCurrentMoveVector)) 0.1)
        (Variables|Default|SetIsRolling true)
        (Development|PrintText (Utilities|Text|ToText(Float) (.x _currentmovevector) "HalfToEven") true true "(R=0.000000,G=0.660000,B=1.000000,A=1.000000)" 1e+01)
        (Transformation|SetActorRotation (Math|Rotator|MakeRotator 0.0 0.0 (+ (+ (.yaw (Pawn|GetControlRotation :!class /Script/Engine.Pawn)) (Math|Trig|RadiansToDegrees (Math|Trig|Atan2(Radians) (.y _currentmovevector) (* (.x _currentmovevector) -1.0)))) -9e+01)))
        (bind _returnvalue (Animation|PlayAnimMontage "/Game/Animations/Player_FrontRoll_Anim_Montage.Player_FrontRoll_Anim_Montage" 1.0 "None"))
        (bind _output_get (Variables|Default|SetRollAnimetionTime _returnvalue))
        (CallFunction|SetIsRollingDelay)
        (Utilities|FlowControl|Delay _output_get)
        (goto _label Reset)))))

(event Input|EnhancedActionEvents|EnhancedInputActionIA_Target
  (params (ActionValue :type Boolean) (ElapsedSeconds :type Float%20%28double-precision%29) (TriggeredSeconds :type Float%20%28double-precision%29) (InputAction :type Input%20Action%20Object%20Reference :default "/Game/Input/IA_Target.IA_Target"))
  (bind _returnvalue (Transformation|GetActorLocation))
  (bind _mesh (Variables|Character|GetMesh))
  (bind _returnvalue_2 (Components|SkeletalMesh|GetAnimInstance _mesh))
  ;[0.15 0.15 0.15 0.5] Target system
  (if (Variables|Default|GetIsTargeting)
    (bind _asplayer_abp (Utilities|Casting|CastToPlayer_ABP _returnvalue_2 :!label _label))
    (Variables|/Game/Blueprint/Player_ABP.Player_ABP_C|SetIsLocked _asplayer_abp false)
    (Variables|Default|SetIsTargeting false)
    (Variables|/Script/Engine.CharacterMovementComponent|SetbOrientRotationToMovement (Variables|Character|GetCharacterMovement) true)
    (Variables|Default|SetCurrentTarget 0)
    (else
      (bind _asplayer_abp_2 (Utilities|Casting|CastToPlayer_ABP _returnvalue_2))
      (bind _outhit (Collision|SphereTraceForObjects _returnvalue (+ _returnvalue (* (Math|Vector|GetForwardVector (Transformation|GetWorldRotation (Variables|Default|GetCamera))) (Variables|Default|GetTargetLocationRange))) (Variables|Default|GetTargetLocationWidth) (Utilities|Array|MakeArray "ObjectTypeQuery3") false 0 "ForDuration"))
      (if (Utilities|IsValid (.HitActor (Collision|BreakHitResult _outhit)))
        (Variables|/Game/Blueprint/Player_ABP.Player_ABP_C|SetIsLocked _asplayer_abp_2 true)
        (Variables|Default|SetIsTargeting true)
        (Variables|/Script/Engine.CharacterMovementComponent|SetbOrientRotationToMovement (Variables|Character|GetCharacterMovement) false)
        (Variables|Default|SetCurrentTarget (.HitActor (Collision|BreakHitResult _outhit)))
        (else
          (goto _label))))))

(event EventBeginPlay
  ;[0.15 0.15 0.15 0.5] Set Mapping Context
  (bind _returnvalue (Sequencer|Player|CreateLevelSequencePlayer "/Game/Animations/Enemy_Animations_LS.Enemy_Animations_LS"))
  (Variables|Default|SetNewVar_0 _returnvalue)
  (Utilities|Time|SetTimerbyFunctionName 0 "PlayMyAnimation" 3.0 true)
  (bind _asplayer_controller (Utilities|Casting|CastToPlayerController (Pawn|GetController)))
  (Utilities|IsValid (PlayerController|LocalPlayerSubsystems|GetEnhancedInputLocalPlayerSubsystem _asplayer_controller)
    (:Is%20Valid
      (Input|AddMappingContext (PlayerController|LocalPlayerSubsystems|GetEnhancedInputLocalPlayerSubsystem _asplayer_controller) "/Game/Input/IMC_Player.IMC_Player" 0 "(bIgnoreAllPressedKeysUntilRelease=True,bForceImmediately=False,bNotifyUserSettings=False)"))))

(event EventTick
  (params (DeltaSeconds :type Float%20%28single-precision%29))
  (bind _returnvalue (Pawn|GetController))
  (bind _returnvalue_2 (Transformation|GetActorLocation))
  (bind _currenttarget (Variables|Default|GetCurrentTarget))
  (bind _returnvalue_3 (Transformation|GetActorLocation _currenttarget))
  (bind _returnvalue_4 (Math|Rotator|FindLookatRotation _returnvalue_2 _returnvalue_3))
  ;[0.15 0.15 0.15 0.5] Event tik
  (CallFunction|UpdateCurrentRotations)
  (Variables|Default|GetCurrentTarget
    (:then
      (if (Variables|Default|GetIsTargeting)
        (if (Variables|Default|GetIsRolling)
          (Pawn|SetControlRotation _returnvalue _returnvalue_4)
          (else
            (Transformation|SetActorRotation (Math|Interpolation|RInterpTo (Transformation|GetActorRotation) (Math|Rotator|MakeRotator 0.0 0.0 (.Yaw (Math|Rotator|BreakRotator _returnvalue_4))) DeltaSeconds (Variables|Default|GetRotationSpeed)))
            (Pawn|SetControlRotation _returnvalue _returnvalue_4)))))
    (:else)))

(fn ConstructionScript)